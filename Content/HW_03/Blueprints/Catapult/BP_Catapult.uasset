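; Physics-driven catapult actor that launches a cannonball by swinging a constrained arm.
; Shoot changes the PhysicsConstraint's angular orientation target, then restores it after a delay, with a busy flag blocking overlapping shots.
; SpawnCannonball replaces any existing ball with a new BP_Cannonball at the spawn point and gives it a back-reference to the catapult.
; It runs shortly after BeginPlay, while Shoot itself does not reload.
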(event Custom|Shoot
  ;[1 1 1] Реализуйте механику выстрела
  (if (not (Variables|Default|GetIsBusy))
    (Variables|Default|SetIsBusy true)
    (Class|PhysicsConstraintComponent|SetAngularOrientationTarget (Variables|Default|GetPhysicsConstraint) (Math|Rotator|MakeRotator -3e+01 0.0 0.0))
    (Utilities|FlowControl|Delay 2.0)
    (Class|PhysicsConstraintComponent|SetAngularOrientationTarget (Variables|Default|GetPhysicsConstraint) (Math|Rotator|MakeRotator 5e+01 0.0 0.0))
    (Variables|Default|SetIsBusy false)))

(event Custom|SpawnCannonball
  (Variables|Default|GetCannonball
    (:then
      (bind _asactor (Utilities|Casting|CastToActor (Variables|Default|GetCannonball)))
      (Actor|DestroyActor _asactor))
    (:else
      _))
  (bind _returnvalue (Game|SpawnActorfromClass "/Game/HW_03/Blueprints/Cannonball/BP_Cannonball.BP_Cannonball_C" (Transformation|GetWorldTransform (Variables|Default|GetCannonballSpawnPoint)) "Undefined" "MultiplyWithRoot" 0 0))
  (bind _output_get (Variables|Default|SetCannonball _returnvalue))
  (bind _asbp_cannonball (Utilities|Casting|CastToBP_Cannonball _output_get))
  (Variables|/Game/HW_03/Blueprints/Cannonball/BP_Cannonball.BP_Cannonball_C|SetCatapult _asbp_cannonball self))

(event EventBeginPlay
  (Utilities|FlowControl|Delay 0.3)
  (CallFunction|SpawnCannonball))

(fn ConstructionScript)